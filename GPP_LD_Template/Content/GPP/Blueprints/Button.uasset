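; Interactable button actor that lets the player trigger a referenced platform.
; Overlap events on the Haha component detect BP_PlayerCharacter, setting an interact flag and showing or hiding a ButtonUI widget created on BeginPlay.
; With input enabled for the first player controller, pressing E while the flag is set calls ButtonPress on the platform reference, then destroys the Haha component.
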(event `self.ReceiveBeginPlay`
  (bind _returnvalue (`|CreateWidget` "/Game/GPP/Blueprints/ButtonUI.ButtonUI_C"))
  (set `self.Button` _returnvalue)
  (`self.EnableInput` (`GameplayStatics.GetPlayerController` 0)))

(event `Key|E`
  (params (Key :type "Key Structure"))
  (:`Pressed`
    (if (`self.Interacttt`)
      (`/Game/GPP/Blueprints/Platforms/BP_ButtonPressPlatform.ButtonPress` (`self.platformref`))
      (`ActorComponent.K2_DestroyComponent` (`self.haha`)))))

(event `self.haha.OnComponentBeginOverlap`
  (params (OverlappedComponent :type "PrimitiveComponent Object Reference") (OtherActor :type "Actor Object Reference") (OtherComp :type "PrimitiveComponent Object Reference") (OtherBodyIndex :type Integer) (bFromSweep :type Boolean) (SweepResult :type "HitResult Structure (by ref)"))
  (cast `/Game/GPP/Blueprints/Essential/BP_PlayerCharacter` OtherActor)
  (set `self.Interacttt` true)
  (`UserWidget.AddToViewport` (`self.Button`) 0))

(event `self.haha.OnComponentEndOverlap`
  (params (OverlappedComponent :type "PrimitiveComponent Object Reference") (OtherActor :type "Actor Object Reference") (OtherComp :type "PrimitiveComponent Object Reference") (OtherBodyIndex :type Integer))
  (cast `/Game/GPP/Blueprints/Essential/BP_PlayerCharacter` OtherActor)
  (set `self.Interacttt` false)
  (`Widget.RemoveFromParent` (`self.Button`)))

(fn `UserConstructionScript`)