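; DoorButton is an interactable button actor that triggers changes on a referenced door and rock.
; Its Hehe overlap component sets an interact flag and shows or removes a ButtonUI prompt as BP_PlayerCharacter enters or leaves.
; It enables input for the first player controller on BeginPlay, so a gamepad right trigger press while in range calls DoorVisible and RockVisible on those references.
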(event `Key|Gamepad_RightTrigger`
  (params (Key :type "Key Structure"))
  (:`Pressed`
    (if (`self.OtherInteract`)
      (`/Game/GPP/Blueprints/Door.DoorVisible` (`self.DoorRef`))
      (`/Game/GPP/Blueprints/Rock.RockVisible` (`self.Rockref`)))))

(event `self.ReceiveBeginPlay`
  (bind _returnvalue (`|CreateWidget` "/Game/GPP/Blueprints/ButtonUI.ButtonUI_C"))
  (set `self.Button` _returnvalue)
  (`self.EnableInput` (`GameplayStatics.GetPlayerController` 0)))

(event `self.hehe.OnComponentBeginOverlap`
  (params (OverlappedComponent :type "PrimitiveComponent Object Reference") (OtherActor :type "Actor Object Reference") (OtherComp :type "PrimitiveComponent Object Reference") (OtherBodyIndex :type Integer) (bFromSweep :type Boolean) (SweepResult :type "HitResult Structure (by ref)"))
  (cast `/Game/GPP/Blueprints/Essential/BP_PlayerCharacter` OtherActor)
  (set `self.OtherInteract` true)
  (`UserWidget.AddToViewport` (`self.Button`) 0))

(event `self.hehe.OnComponentEndOverlap`
  (params (OverlappedComponent :type "PrimitiveComponent Object Reference") (OtherActor :type "Actor Object Reference") (OtherComp :type "PrimitiveComponent Object Reference") (OtherBodyIndex :type Integer))
  (cast `/Game/GPP/Blueprints/Essential/BP_PlayerCharacter` OtherActor)
  (set `self.OtherInteract` false)
  (`Widget.RemoveFromParent` (`self.Button`)))

(fn `UserConstructionScript`)